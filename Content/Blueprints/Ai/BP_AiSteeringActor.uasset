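; AI steering actor that, as shown, only wires up physics and health and logs health events.
; On BeginPlay it sets its Billboard as the Physics component's angular body and binds to the Health component's damage and change events.
; Both handlers print debug messages with the actor's name and current health.
; DrawDebugCompass is a stub: its debug-line loop is disconnected and never runs.
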(event `self.ReceiveBeginPlay`
  (bind _health (`self.Health`))
  (`NetworkedPhysics.SetAngularBody` (`self.Physics`) (`self.Billboard`))
  (add `HealthComponent.OnTakeDamage` _health (delegate `TakeDamageEvent`))
  (add `HealthComponent.OnHealthChanged` _health (delegate `EventHealthUpdate`)))

(event `TakeDamageEvent`
  (params (DamageValue :type "Float (single-precision)") (NewHealth :type "Float (single-precision)"))
  (`KismetSystemLibrary.PrintString` (`KismetStringLibrary.Concat_StrStr` (`KismetSystemLibrary.GetDisplayName` self) " took" (`KismetStringLibrary.Conv_DoubleToString` DamageValue) " damage. Health = " (`KismetStringLibrary.Conv_DoubleToString` NewHealth)) true true (struct :`G` 0.66 :`B` 1.0 :`A` 1.0) 10.0))

(event `EventHealthUpdate`
  (bind _returnvalue (`HealthComponent.GetHealth` (`self.Health`)))
  (`KismetSystemLibrary.PrintString` (`KismetStringLibrary.Concat_StrStr` (`KismetSystemLibrary.GetDisplayName` self) " health was changed. Health = " (`KismetStringLibrary.Conv_DoubleToString` _returnvalue)) true true (struct :`G` 1.0 :`B` 0.045961 :`A` 1.0) 10.0))

(fn `DrawDebugCompass`)

(fn `UserConstructionScript`)