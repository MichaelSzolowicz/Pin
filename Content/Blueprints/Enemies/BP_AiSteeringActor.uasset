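; AI steering enemy actor with Health, Movement and Steering components that bounces off what it hits and logs health changes.
; Sphere hits add a horizontal impulse along the hit normal to Movement, skipping BlockAllDynamic components and throttled by a short dummy timer.
; Health delegates print damage taken and current health on screen.
; Debug helpers for the steering compass and speed exist but are not run, and Tick is empty.
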(event `self.ReceiveBeginPlay`
  (bind _health (`self.Health`))
  (add `HealthComponent.OnTakeDamage` _health (delegate `TakeDamageEvent`))
  (add `HealthComponent.OnHealthChanged` _health (delegate `EventHealthUpdate`)))

(event `TakeDamageEvent`
  (params (DamageValue :type "Float (single-precision)") (NewHealth :type "Float (single-precision)"))
  (`self.PrintDamageTaken` DamageValue NewHealth))

(event `EventHealthUpdate`
  (`self.PrintCurrentHealth`))

(event `self.ReceiveTick`
  (params (DeltaSeconds :type "Float (single-precision)")))

(event `self.Sphere.OnComponentHit`
  (params (HitComponent :type "PrimitiveComponent Object Reference") (OtherActor :type "Actor Object Reference") (OtherComp :type "PrimitiveComponent Object Reference") (NormalImpulse :type "Vector Structure") (Hit :type "HitResult Structure (by ref)"))
  (if (not (`KismetSystemLibrary.K2_IsTimerActiveHandle` (`self.Timer`)))
    (bind _returnvalue (`KismetSystemLibrary.K2_SetTimerDelegate` (delegate `Dummy`) 0.1))
    (set `self.Timer` _returnvalue)
    (`self.AddFixedNormalImpulse` OtherComp Hit 999.0)))

(event `Dummy`)

(fn `AddFixedNormalImpulse`
  (params (self2 :type "PrimitiveComponent Object Reference") (Hit :type "HitResult Structure (by ref)") (Scale :type "Float (double-precision)"))
  (if (!= (`PrimitiveComponent.GetCollisionProfileName` self2) "BlockAllDynamic")
    (`EnemyMovement.AddImpulse` (`self.Movement`) (* Scale (`KismetMathLibrary.MakeVector` (.x (`.Normal` (`GameplayStatics.BreakHitResult` Hit))) (.y (`.Normal` (`GameplayStatics.BreakHitResult` Hit))))))
    (`KismetSystemLibrary.PrintString` "Hello" true true (struct :`R` 1.0 :`G` 0.210431 :`A` 1.0))))

(fn `DrawDebugCompass`
  (bind _returnvalue (`self.K2_GetActorLocation`))
  (bind _returnvalue_2 (`AiSteering.GetCompass` (`self.Steering`)))
  (for _array_element _returnvalue_2
    (`KismetSystemLibrary.DrawDebugLine` _returnvalue (+ _returnvalue (* _array_element (0.0 0.0 0.0))) (struct :`G` 1.0 :`A` 1.0) 0.01 1.0)))

(fn `PrintCurrentHealth`
  (bind _returnvalue (`HealthComponent.GetHealth` (`self.Health`)))
  (`KismetSystemLibrary.PrintString` (`KismetStringLibrary.Concat_StrStr` (`KismetSystemLibrary.GetDisplayName` self) " health was changed. Health = " (`KismetStringLibrary.Conv_DoubleToString` _returnvalue)) true true (struct :`G` 1.0 :`B` 0.045961 :`A` 1.0) 10.0))

(fn `PrintDamageTaken`
  (params (InDouble :type "Float (double-precision)") (InDouble2 :type "Float (double-precision)"))
  (`KismetSystemLibrary.PrintString` (`KismetStringLibrary.Concat_StrStr` (`KismetSystemLibrary.GetDisplayName` self) " took" (`KismetStringLibrary.Conv_DoubleToString` InDouble) " damage. Health = " (`KismetStringLibrary.Conv_DoubleToString` InDouble2)) true true (struct :`G` 0.66 :`B` 1.0 :`A` 1.0) 10.0))

(fn `PrintSpeed`
  (bind _movement (`self.Movement`))
  (`KismetSystemLibrary.PrintString` (`KismetStringLibrary.Conv_DoubleToString` (`KismetMathLibrary.VSize` (+ (`EnemyMovement.ExternalVelocity` _movement) (`EnemyMovement.ControlVelocity` _movement))))))

(fn `UserConstructionScript`)