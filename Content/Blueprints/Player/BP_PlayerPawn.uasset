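; Player pawn that moves by applying input-driven force on the horizontal plane and fires a grapple projectile.
; Tick scales X/Y input by ForceStrength into the PlayerPhysics component, which also spawns and despawns the grapple on Space press and release.
; On clients, the GrappleProj RepNotify snaps the replicated projectile to the local stand-in's location, then destroys the stand-in.
; The SayHi action multiplies ForceStrength fivefold on clients only.
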(event `InputAction|SayHi`
  (params (Key :type "Key Structure"))
  (:`Pressed`
    (`/Engine/EditorBlueprintResources/ActorMacros.Switch Has Authority`
      (:`Remote`
        (set `self.ForceStrength` (* (`self.ForceStrength`) 5.0))))))

(event `Key|SpaceBar`
  (params (Key :type "Key Structure"))
  (bind _playerphysics (`self.PlayerPhysics`))
  (:`Pressed`
    (`PlayerPhysics.SpawnGrappleProjectile` _playerphysics))
  (:`Released`
    (`PlayerPhysics.DespawnGrappleProjectile` _playerphysics)))

(event `self.ReceiveTick`
  (params (DeltaSeconds :type "Float (single-precision)"))
  (bind _forcestrength (`self.ForceStrength`))
  (`NetworkedPhysics.AddForce` (`self.PlayerPhysics`) (* (`KismetMathLibrary.MakeVector` (`self.GetInputAxisValue`) (`self.GetInputAxisValue`)) (`KismetMathLibrary.MakeVector` _forcestrength _forcestrength))))

(fn `OnRep_GrappleProj`
  (bind _grappleprojlocal (`self.GrappleProjLocal`))
  (`/Engine/EditorBlueprintResources/ActorMacros.Switch Has Authority`
    (:`Remote`
      (if (`KismetSystemLibrary.IsValid` _grappleprojlocal)
        (`self.K2_SetActorLocation` (`self.GrappleProj`) (`self.K2_GetActorLocation` _grappleprojlocal) false false)
        (`self.K2_DestroyActor` _grappleprojlocal)))))

(fn `UserConstructionScript`)