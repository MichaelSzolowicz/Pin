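; Pinball camera that finds the first BP_PinballPlayer at BeginPlay and adjusts its view to that player's speed.
; Each tick it passes the magnitude of the player's NetworkPhysics velocity to SpeedRelativeControls.
; That component interpolates the spring arm's world pitch using the CF_CameraSpeedRotation curve, leaving yaw and roll unchanged.
; CameraPositionVolume then updates its position every frame.
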(event `self.ReceiveBeginPlay`
  (bind _outactors (`GameplayStatics.GetAllActorsOfClass` "/Game/Blueprints/Player/BP_PinballPlayer.BP_PinballPlayer_C"))
  (set `self.Player` (`|GetArrayItem` _outactors)))

(event `self.ReceiveTick`
  (params (DeltaSeconds :type "Float (single-precision)"))
  (set `CameraSpeedRelativeControls.Speed` (`KismetMathLibrary.VSize` (`NetworkedPhysics.LinearVelocity` (`PinballPlayer.NetworkPhysics` (`self.Player`)))) (`self.SpeedRelativeControls`))
  (`self.UpdateCameraSpeedRotation` DeltaSeconds)
  (`CameraPositionVolume.UpdatePosition` (`self.CameraPositionVolume`)))

(fn `UpdateCameraSpeedRotation`
  (params (DeltaTime :type "Float (single-precision)"))
  (locals (RotationCurve :type "CurveFloat Object Reference" :default "/Script/Engine.CurveFloat'/Game/Blueprints/Player/CF_CameraSpeedRotation.CF_CameraSpeedRotation'"))
  (bind _springarm (`self.SpringArm`))
  (bind (_returnvalue_roll _returnvalue_pitch _returnvalue_yaw) (`KismetMathLibrary.BreakRotator` (`SceneComponent.K2_GetComponentRotation` _springarm)))
  (bind _returnvalue (`CameraSpeedRelativeControls.InterpolateTowards` (`self.SpeedRelativeControls`) "/Game/Blueprints/Player/CF_CameraSpeedRotation.CF_CameraSpeedRotation" _returnvalue_pitch DeltaTime))
  (`SceneComponent.K2_SetWorldRotation` _springarm (`KismetMathLibrary.MakeRotator` _returnvalue_roll _returnvalue _returnvalue_yaw) false false))

(fn `UserConstructionScript`)