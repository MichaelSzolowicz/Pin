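; BP_TestProjectile is a test projectile that sticks to the first or any later actor its mesh overlaps.
; On overlap, it sets that actor as the StickyProjectile's AttachedTo, zeroes its Speed and prints the actor's name.
; On BeginPlay without authority, it passes its location to the SetupServer event, which sets the actor location and prints a debug message.
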(event `self.ReceiveBeginPlay`
  (`/Engine/EditorBlueprintResources/ActorMacros.Switch Has Authority`
    (:`Remote`
      (`self.SetupServer` (`self.K2_GetActorLocation`)))))

(event `SetupServer`
  (params (NewLocation :type "Vector Structure"))
  (`self.K2_SetActorLocation` NewLocation)
  (`KismetSystemLibrary.PrintString` "Hello"))

(event `self.StaticMesh.OnComponentBeginOverlap`
  (params (OverlappedComponent :type "PrimitiveComponent Object Reference") (OtherActor :type "Actor Object Reference") (OtherComp :type "PrimitiveComponent Object Reference") (OtherBodyIndex :type Integer) (bFromSweep :type Boolean) (SweepResult :type "HitResult Structure (by ref)"))
  (bind _stickyprojectile (`self.StickyProjectile`))
  (set `StickyProjectile.AttachedTo` OtherActor _stickyprojectile)
  (set `SimpleProjectile.Speed` 0.0 _stickyprojectile)
  (`KismetSystemLibrary.PrintString` (`KismetSystemLibrary.GetDisplayName` OtherActor)))

(fn `UserConstructionScript`)