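; Game mode for local multiplayer that creates player controllers and spawns a possessed BP_PlayerPawn for each player index at its matching BP_PlayerStart.
; On BeginPlay it sets up the first controller as player 0, then creates local players from the current player count through MaxPlayerIndex where matching starts exist.
; InitPlayerPawn spawns each pawn at that start, assigns its index and possesses it, while controllers created later and all pawns are tracked in arrays.
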(event `self.ReceiveBeginPlay`
  (`self.InitPlayerPawn` (`GameplayStatics.GetPlayerController` 0))
  (`self.SpawnRemainingPlayers`))

(event `self.SpawnRemainingPlayers`
  (`self.CreateAllPlayerControllers`))

(fn `CreateAllPlayerControllers`
  (locals (PlayerStartArray :type "Array of /Game/Blueprints/Player/BP_PlayerStart Object Reference"))
  (bind _outactors (`GameplayStatics.GetAllActorsOfClass` "/Game/Blueprints/Player/BP_PlayerStart.BP_PlayerStart_C"))
  (set `local.PlayerStartArray` _outactors)
  (bind _returnvalue (`self.GetNumPlayers`))
  (for _index (range _returnvalue (+ (`self.MaxPlayerIndex`) 1))
    (for _array_element (`local.PlayerStartArray`)
      (bind _playerindex (`PinPlayerStart.PlayerIndex` _array_element))
      (if (== _playerindex _index)
        (bind _returnvalue_2 (`GameplayStatics.CreatePlayer` -1))
        (bind _asbp_player_controller (cast `/Game/Blueprints/Player/BP_PlayerController` _returnvalue_2))
        (`KismetArrayLibrary.Array_AddUnique` (`self.PlayerControllerArray`) _asbp_player_controller)
        (`self.InitPlayerPawn` _asbp_player_controller _playerindex)))))

(fn `InitPlayerPawn`
  (params (NewController :type "Controller Object Reference") (PlayerIndex :type Integer))
  (locals (PlayerStarts :type "Array of /Game/Blueprints/Player/BP_PlayerStart Object Reference"))
  (bind _outactors (`GameplayStatics.GetAllActorsOfClass` "/Game/Blueprints/Player/BP_PlayerStart.BP_PlayerStart_C"))
  (bind _output_get (set `local.PlayerStarts` _outactors))
  (for _array_element _output_get
    (if (== (`PinPlayerStart.PlayerIndex` _array_element) (`local.PlayerIndex`))
      (bind _returnvalue (`|SpawnActorFromClass` "/Game/Blueprints/Player/BP_PlayerPawn.BP_PlayerPawn_C" (`self.GetTransform` _array_element) "Undefined" "OverrideRootScale" null null))
      (`KismetArrayLibrary.Array_AddUnique` (`self.PlayerPawnArray`) _returnvalue)
      (`PinPlayerPawn.SetPlayerIndex` _returnvalue (`local.PlayerIndex`))
      (`Controller.Possess` (`local.NewController`) _returnvalue))))

(fn `UserConstructionScript`)